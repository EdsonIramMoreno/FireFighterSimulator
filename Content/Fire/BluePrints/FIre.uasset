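; Fire actor that the VR player puts out with a hose, turning to smoke once its life runs out.
; BeginPlay spawns a fire sound at its location, chosen by the current level name, and keeps a reference to it.
; MakeFireDamage subtracts the VRPawn's HosePower from FireLife.
; Tick polls FireLife and, at zero or below, briefly delays, spawns Smoke, then destroys the sound and the actor.
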(event EventBeginPlay
  (bind _self self)
  (bind _returnvalue (Transformation|GetActorLocation _self))
  (bind _returnvalue_2 (Game|GetCurrentLevelName true))
  (if (Utilities|Enum|Equal(Enum) _returnvalue_2 "Nivel_1")
    (bind _returnvalue_3 (Audio|SpawnSoundatLocation "/Game/sound/fire/ES_Fire_Auto_-_SFX_Producer.ES_Fire_Auto_-_SFX_Producer" _returnvalue "0, 0, 0" 1.0 1.0 0.0 0 0))
    (Variables|Default|SetFireSound _returnvalue_3)
    (elif (Utilities|Enum|Equal(Enum) _returnvalue_2 "Nivel_2")
      (bind _returnvalue_4 (Audio|SpawnSoundatLocation "/Game/sound/fire/ES_Gas_Flame_Loop_-_SFX_Producer.ES_Gas_Flame_Loop_-_SFX_Producer" _returnvalue "0, 0, 0" 1.0 1.0 0.0 0 0))
      (Variables|Default|SetFireSound _returnvalue_4)
      (else
        (bind _returnvalue_5 (Audio|SpawnSoundatLocation "/Game/sound/fire/ES_Fire_Fireplace_1_-_SFX_Producer.ES_Fire_Fireplace_1_-_SFX_Producer" _returnvalue "0, 0, 0" 1.0 1.0 0.0 0 0))
        (Variables|Default|SetFireSound _returnvalue_5)))))

(event EventTick
  (params (DeltaSeconds :type Float%20%28single-precision%29))
  (if (<= (Variables|Default|GetFire_Life) 0.0)
    (Utilities|FlowControl|Delay 0.2)
    (Game|SpawnActorfromClass "/Game/Fire/BluePrints/Smoke.Smoke_C" (Transformation|GetActorTransform self) "Undefined" 0 0)
    (Components|DestroyComponent (Variables|Default|GetFireSound))
    (Actor|DestroyActor)))

(fn ConstructionScript)

(fn MakeFireDamage
  (bind _asvrpawn (Utilities|Casting|CastToVRPawn (Game|Player|GetPlayerPawn 0)))
  (Variables|Default|SetFire_Life (- (Variables|Default|GetFire_Life) (Variables|/Game/VRTemplate/Blueprints/VRPawn.VRPawn_C|GetHosePower _asvrpawn))))