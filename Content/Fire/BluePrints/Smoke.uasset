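; Short-lived smoke actor that spawns a HumoBlanco particle emitter at its own location when play begins.
; It checks the current level name for Nivel_1 and Nivel_2, but every branch spawns the same emitter.
; After a ten-second delay the actor destroys itself.
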(event EventBeginPlay
  (bind _self self)
  (bind _returnvalue (Transformation|GetActorLocation _self))
  (bind _returnvalue_2 (Game|GetCurrentLevelName true))
  (if (Utilities|Enum|Equal(Enum) _returnvalue_2 "Nivel_1")
    (Effects|SpawnEmitteratLocation "/Game/Fire/HumoBlanco.HumoBlanco" _returnvalue)
    (elif (Utilities|Enum|Equal(Enum) _returnvalue_2 "Nivel_2")
      (Effects|SpawnEmitteratLocation "/Game/Fire/HumoBlanco.HumoBlanco" _returnvalue)
      (else
        (Effects|SpawnEmitteratLocation "/Game/Fire/HumoBlanco.HumoBlanco" _returnvalue))))
  (Utilities|FlowControl|Delay 1e+01)
  (Actor|DestroyActor))

(fn ConstructionScript)